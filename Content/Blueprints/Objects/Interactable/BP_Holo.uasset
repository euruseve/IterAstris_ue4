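; BP_Holo is an interactable hologram object that starts a Mountea dialogue when the player interacts with it.
; Its interaction widget is shown only when the dialogue participant component has a dialogue graph assigned, and is hidden on request.
; Interact initializes the dialogue with itself as initiator and its own participant component.
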(event `InteractionInterface.ShowInteractionWidget`
  (if (!= (`MounteaDialogueParticipant.GetDialogueGraph` (`self.MounteaDialogueParticipant`)) null)
    (`SceneComponent.SetVisibility` (`self.InteractionWidget`) true false)))

(event `InteractionInterface.HideInteractionWidget`
  (`SceneComponent.SetVisibility` (`self.InteractionWidget`) false false))

(event `InteractionInterface.Interact`
  (`MounteaDialogueSystemBFC.InitializeDialogue` self (`self.MounteaDialogueParticipant`)))

(fn `UserConstructionScript`)