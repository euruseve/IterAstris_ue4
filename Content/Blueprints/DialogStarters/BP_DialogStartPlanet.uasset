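; Dialogue starter actor that plays a Mountea dialogue the first time the planet flag is set in the game instance.
; On BeginPlay it checks and clears IsFirstTimePlanet on GI_Main, then after a short delay initializes dialogue with itself as initiator and its participant component.
; When that participant's state changes to Enabled, it closes the dialogue.
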(event `self.ReceiveBeginPlay`
  (bind _asgi_main (cast `/Game/GI_Main` (`GameplayStatics.GetGameInstance`)))
  (if (`/Game/GI_Main.bIsFirstTimePlanet` _asgi_main)
    (set `/Game/GI_Main.bIsFirstTimePlanet` false _asgi_main)
    (`KismetSystemLibrary.Delay` 1.0)
    (`MounteaDialogueSystemBFC.InitializeDialogue` self (`self.MounteaDialogueParticipant`))))

(event `self.MounteaDialogueParticipant.OnDialogueParticipantStateChanged`
  (params (NewState :type "EDialogueParticipantState Enum (by ref)" :default "EDPS_Disabled"))
  (switch `EDialogueParticipantState` NewState
    (:`EDPS_Enabled`
      (`MounteaDialogueSystemBFC.CloseDialogue` (`self.MounteaDialogueParticipant`)))))

(fn `UserConstructionScript`)