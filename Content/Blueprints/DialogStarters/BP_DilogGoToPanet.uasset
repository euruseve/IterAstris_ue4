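; One-shot trigger volume that starts a dialogue for the player's first trip to the planet.
; Any Box overlap checks IsToPlanetFirstTime on GI_Main, clears it, then after a short delay initializes a Mountea dialogue with itself as initiator and its participant component.
; Keeping the flag in the game instance stops replays across level loads.
; When the participant's state changes to Enabled, it calls CloseDialogue on that participant.
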(event `self.ReceiveBeginPlay`)

(event `self.Box.OnComponentBeginOverlap`
  (params (OverlappedComponent :type "PrimitiveComponent Object Reference") (OtherActor :type "Actor Object Reference") (OtherComp :type "PrimitiveComponent Object Reference") (OtherBodyIndex :type Integer) (bFromSweep :type Boolean) (SweepResult :type "HitResult Structure (by ref)"))
  (bind _asgi_main (cast `/Game/GI_Main` (`GameplayStatics.GetGameInstance`)))
  (if (`/Game/GI_Main.bIsToPlanetFirstTime` _asgi_main)
    (set `/Game/GI_Main.bIsToPlanetFirstTime` false _asgi_main)
    (`KismetSystemLibrary.Delay` 0.5)
    (`MounteaDialogueSystemBFC.InitializeDialogue` self (`self.MounteaDialogueParticipant`))))

(event `self.MounteaDialogueParticipant.OnDialogueParticipantStateChanged`
  (params (NewState :type "EDialogueParticipantState Enum (by ref)" :default "EDPS_Disabled"))
  (switch `EDialogueParticipantState` NewState
    (:`EDPS_Enabled`
      (`MounteaDialogueSystemBFC.CloseDialogue` (`self.MounteaDialogueParticipant`)))))

(fn `UserConstructionScript`)