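; BP_ChangeLevel is an interactable actor that moves the player to another level.
; Show and hide interaction events toggle the visibility of its InteractionWidget prompt.
; On Interact it stores its TeleportTag in the GI_Main game instance, which persists across the load, then opens the level named by LevelName.
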(event `InteractionInterface.ShowInteractionWidget`
  (`SceneComponent.SetVisibility` (`self.InteractionWidget`) true false))

(event `InteractionInterface.HideInteractionWidget`
  (`SceneComponent.SetVisibility` (`self.InteractionWidget`) false false))

(event `InteractionInterface.Interact`
  (bind _asgi_main (cast `/Game/GI_Main` (`GameplayStatics.GetGameInstance`)))
  (set `/Game/GI_Main.TeleportationTag` (`self.TeleportTag`) _asgi_main)
  (`GameplayStatics.OpenLevel` (`self.Level Name`)))

(fn `UserConstructionScript`)