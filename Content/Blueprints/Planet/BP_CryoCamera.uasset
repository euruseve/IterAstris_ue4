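; BP_CryoCamera runs the one-time cryo room intro, pairing an opening dialogue with a cryo gate animation.
; On BeginPlay it checks and clears a first-play flag on GI_Main, starts the D_CryoRoomStart Mountea dialogue, then plays the gate-opening animation once on CryoCamera after short delays.
; The dialogue closes when its participant's state changes to Enabled.
; A separate DisablePlayerModel function hides the Player component.
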(event `self.ReceiveBeginPlay`
  (bind _asgi_main (cast `/Game/GI_Main` (`GameplayStatics.GetGameInstance`)))
  (if (`/Game/GI_Main.bIsFirstTimePlayCryo` _asgi_main)
    (set `/Game/GI_Main.bIsFirstTimePlayCryo` false _asgi_main)
    (`MounteaDialogueParticipant.SetDialogueGraph` (`self.MounteaDialogueParticipant`) "/Game/Dialogue/DialogTrees/D_CryoRoomStart.D_CryoRoomStart")
    (`KismetSystemLibrary.Delay` 0.01)
    (`MounteaDialogueSystemBFC.InitializeDialogue` self (`self.MounteaDialogueParticipant`))
    (`KismetSystemLibrary.Delay` 0.5)
    (`SkeletalMeshComponent.PlayAnimation` (`self.CryoCamera`) "/Game/_ExternalContent/Objects/Cryo/CryoChamb/cryo_fixed_mb_Anim_cryo_gate_opening_armature_cryo_gate_opening_cryo_gate_opening_cryo_gate_openingAction.cryo_fixed_mb_Anim_cryo_gate_opening_armature_cryo_gate_opening_cryo_gate_opening_cryo_gate_openingAction" false)))

(event `self.MounteaDialogueParticipant.OnDialogueParticipantStateChanged`
  (params (NewState :type "EDialogueParticipantState Enum (by ref)" :default "EDPS_Disabled"))
  (switch `EDialogueParticipantState` NewState
    (:`EDPS_Enabled`
      (`MounteaDialogueSystemBFC.CloseDialogue` (`self.MounteaDialogueParticipant`)))))

(fn `DisablePlayerModel`
  (`SceneComponent.SetVisibility` (`self.Player`) false false))

(fn `UserConstructionScript`)