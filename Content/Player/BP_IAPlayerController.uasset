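; Player controller that handles the SkipDialogue input for Mountea dialogue.
; Press and release each refresh the dialogue widget when it is valid, and press also starts a short one-shot timer.
; DialogueSkipHoldFinished, the apparent timer callback, requests a voice skip from the dialogue manager and tells the widget to hide the skip UI.
; Release does not clear the timer.
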(event `InputAction|SkipDialogue`
  (params (Key :type "Key Structure"))
  (bind _mounteadialoguemanager (`self.MounteaDialogueManager`))
  (bind _returnvalue (`MounteaDialogueManager.GetDialogueUIPtr` (`self.MounteaDialogueManager`)))
  (:`Pressed`
    (`/Engine/EditorBlueprintResources/StandardMacros.IsValid` _returnvalue
      (:`Is Valid`
        (message `MounteaDialogueWBPInterface.RefreshDialogueWidget` _returnvalue _mounteadialoguemanager "")
        (`KismetSystemLibrary.K2_SetTimerDelegate` (`|CreateDelegate` :!event `DialogueSkipHoldFinished`) 0.1))))
  (:`Released`
    (`/Engine/EditorBlueprintResources/StandardMacros.IsValid` _returnvalue
      (:`Is Valid`
        (message `MounteaDialogueWBPInterface.RefreshDialogueWidget` _returnvalue _mounteadialoguemanager "")))))

(fn `DialogueSkipHoldFinished`
  (`MounteaDialogueManager.OnDialogueVoiceSkipRequest` (`self.MounteaDialogueManager`) null)
  (message `MounteaDialogueWBPInterface.RefreshDialogueWidget` (`MounteaDialogueManager.GetDialogueUIPtr` (`self.MounteaDialogueManager`)) (`self.MounteaDialogueManager`) "HideSkipUI"))

(fn `UserConstructionScript`)