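; Dev test actor for an interactable that starts a dialogue through the Mountea dialogue system.
; Show and hide events toggle an interaction widget, with showing gated by a CanInteract flag.
; Interact clears the flag, sets the widget visible and initializes dialogue with itself as initiator and its participant component.
; When the participant's state changes to Enabled, it closes the dialogue and re-enables interaction.
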(event `self.ReceiveBeginPlay`)

(event `self.MounteaDialogueParticipant.OnDialogueParticipantStateChanged`
  (params (NewState :type "EDialogueParticipantState Enum (by ref)" :default "EDPS_Disabled"))
  (switch `EDialogueParticipantState` NewState
    (:`EDPS_Enabled`
      (`MounteaDialogueSystemBFC.CloseDialogue` (`self.MounteaDialogueParticipant`))
      (set `self.bCanInteract` true))))

(event `InteractionInterface.ShowInteractionWidget`
  (if (`self.bCanInteract`)
    (`SceneComponent.SetVisibility` (`self.Widget`) true false)))

(event `InteractionInterface.Interact`
  (if (`self.bCanInteract`)
    (set `self.bCanInteract` false)
    (`SceneComponent.SetVisibility` (`self.Widget`) true false)
    (`MounteaDialogueSystemBFC.InitializeDialogue` self (`self.MounteaDialogueParticipant`))))

(event `InteractionInterface.HideInteractionWidget`
  (`SceneComponent.SetVisibility` (`self.Widget`) false false))

(fn `UserConstructionScript`)